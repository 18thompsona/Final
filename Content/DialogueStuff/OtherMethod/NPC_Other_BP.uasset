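; NPC Blueprint that shows data-table dialogue in the HUD dialogue box when interacted with.
; BeginPlay caches the Dialogue rows matching its NPC ID, and each Interact advances the line counter and shows the row matching the current conversation and line IDs.
; Without exactly one match, it hides the box and resets the counter.
; A retriggerable delay also hides the box after a few seconds without interaction.
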(event EventBeginPlay
  (bind _outrownames (DataTable|GetDataTableRowNames "/Game/DialogueStuff/OtherMethod/Dialogue.Dialogue"))
  (for _array_element _outrownames
    (bind _returnvalue (Utilities|GetDataTableRow "/Game/DialogueStuff/OtherMethod/Dialogue.Dialogue" _array_element)
      (:then
        (if (== (.npc_id _returnvalue) (Variables|Default|GetNPC_ID))
          (Utilities|Array|Add (Variables|Default|GetMyDialogue) _array_element))))))

(event EventInteract
  (Math|Integer|IncrementInt (Variables|Default|GetLineCurrent_ID)
    (:%20%20
      (CallFunction|DialogCreate)
      ;[1 1 1] removes dialouge after set period
      (Utilities|FlowControl|RetriggerableDelay 4.0)
      (bind _asthird_person_game_mode (Utilities|Casting|CastToThirdPersonGameMode (Game|GetGameMode)))
      (Widget|SetVisibility (Variables|/Game/DialogueStuff/UserInterface/HeadsUpDisplay.HeadsUpDisplay_C|GetDialogueBox (Variables|/Game/ThirdPersonBP/Blueprints/ThirdPersonGameMode.ThirdPersonGameMode_C|GetHeadsUpDisplay _asthird_person_game_mode)) "Hidden"))))

(fn ConstructionScript)

(fn DialogCreate
  (bind _isvisible (CallFunction|IsBoxVisible))
  (if _isvisible
    (bind _asthird_person_game_mode (Utilities|Casting|CastToThirdPersonGameMode (Game|GetGameMode)))
    (bind _returnedline (CallFunction|DialogGetLine))
    (Variables|/Game/DialogueStuff/UserInterface/DialogueBox.DialogueBox_C|SetDialogueText (Variables|/Game/DialogueStuff/UserInterface/HeadsUpDisplay.HeadsUpDisplay_C|GetDialogueBox (Variables|/Game/ThirdPersonBP/Blueprints/ThirdPersonGameMode.ThirdPersonGameMode_C|GetHeadsUpDisplay _asthird_person_game_mode)) _returnedline)
    (else
      (bind _asthird_person_game_mode_2 (Utilities|Casting|CastToThirdPersonGameMode (Game|GetGameMode)))
      (Widget|SetVisibility (Variables|/Game/DialogueStuff/UserInterface/HeadsUpDisplay.HeadsUpDisplay_C|GetDialogueBox (Variables|/Game/ThirdPersonBP/Blueprints/ThirdPersonGameMode.ThirdPersonGameMode_C|GetHeadsUpDisplay _asthird_person_game_mode_2)) "Visible")
      (Variables|/Game/DialogueStuff/UserInterface/DialogueBox.DialogueBox_C|SetSpeaker (Variables|/Game/DialogueStuff/UserInterface/HeadsUpDisplay.HeadsUpDisplay_C|GetDialogueBox (Variables|/Game/ThirdPersonBP/Blueprints/ThirdPersonGameMode.ThirdPersonGameMode_C|GetHeadsUpDisplay _asthird_person_game_mode_2)) (Variables|Default|GetSpeakerName))
      (bind _returnedline_2 (CallFunction|DialogGetLine))
      (Variables|/Game/DialogueStuff/UserInterface/DialogueBox.DialogueBox_C|SetDialogueText (Variables|/Game/DialogueStuff/UserInterface/HeadsUpDisplay.HeadsUpDisplay_C|GetDialogueBox (Variables|/Game/ThirdPersonBP/Blueprints/ThirdPersonGameMode.ThirdPersonGameMode_C|GetHeadsUpDisplay _asthird_person_game_mode_2)) _returnedline_2))))

(fn DialogGetLine
  (for _array_element (Variables|Default|GetMyDialogue)
    ;[1 1 1] Duplicate Protection and Assureing the right line is used
    (bind _returnvalue (Utilities|GetDataTableRow "/Game/DialogueStuff/OtherMethod/Dialogue.Dialogue" _array_element)
      (:then
        (if (and (== (.conversation_id _returnvalue) (Variables|Default|GetConversation_ID)) (== (.line_id _returnvalue) (Variables|Default|GetLineCurrent_ID)))
          (Utilities|Array|Add (LocalVariables|GetReturnedLines) (.dialogue _returnvalue))))))
  (if (== (Utilities|Array|Length (LocalVariables|GetReturnedLines)) 1)
    (return (Utilities|Array|Get(acopy) (LocalVariables|GetReturnedLines)))
    (else
      ;[1 1 1] End to Dialogue
      (bind _asthird_person_game_mode (Utilities|Casting|CastToThirdPersonGameMode (Game|GetGameMode)))
      (Widget|SetVisibility (Variables|/Game/DialogueStuff/UserInterface/HeadsUpDisplay.HeadsUpDisplay_C|GetDialogueBox (Variables|/Game/ThirdPersonBP/Blueprints/ThirdPersonGameMode.ThirdPersonGameMode_C|GetHeadsUpDisplay _asthird_person_game_mode)) "Hidden")
      ;;[1 1 1] Resets the Dialogue
      (Variables|Default|SetLineCurrent_ID 0)
      (return ""))))

(fn IsBoxVisible
  (bind _asthird_person_game_mode (Utilities|Casting|CastToThirdPersonGameMode (Game|GetGameMode)))
  (return (Widget|IsVisible (Variables|/Game/DialogueStuff/UserInterface/HeadsUpDisplay.HeadsUpDisplay_C|GetDialogueBox (Variables|/Game/ThirdPersonBP/Blueprints/ThirdPersonGameMode.ThirdPersonGameMode_C|GetHeadsUpDisplay _asthird_person_game_mode)))))